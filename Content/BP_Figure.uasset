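; BP_Figure is an actor that outlines a closed figure through the actors in its FigureDots array.
; Every Tick, once at least two dots exist, it draws a red debug line from each dot's location to the next, wrapping the last back to the first.
; Positions are read live, so the outline follows any movement of the dots.
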(event `self.ReceiveBeginPlay`)

(event `self.ReceiveTick`
  (params (DeltaSeconds :type "Float (single-precision)"))
  (bind _figuredots (`self.FigureDots`))
  (if (>= (`KismetArrayLibrary.Array_Length` _figuredots) 2)
    (for (_array_element _array_index) _figuredots
      (if (< _array_index (- (`KismetArrayLibrary.Array_Length` (`self.FigureDots`)) 1))
        (`KismetSystemLibrary.DrawDebugLine` (`self.K2_GetActorLocation` _array_element) (`self.K2_GetActorLocation` (`|GetArrayItem` (`self.FigureDots`) (+ _array_index 1))) (struct :`R` 0.953125 :`B` 0.00734 :`A` 1.0) 0.0 5.0)
        (else
          (`KismetSystemLibrary.DrawDebugLine` (`self.K2_GetActorLocation` _array_element) (`self.K2_GetActorLocation` (`|GetArrayItem` (`self.FigureDots`))) (struct :`R` 0.953125 :`B` 0.00734 :`A` 1.0) 0.0 5.0))))))

(fn `UserConstructionScript`)